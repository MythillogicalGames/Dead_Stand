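; Door actor, named as destructible, that the player swings open and closed with the ActionButton input.
; Its TriggerVolume enables player 0's input on any begin overlap and disables it on end overlap.
; Each press flips DoorPos and plays or reverses a timeline whose Driver value, added to CurrentRot, sets the actor's relative yaw.
; IsDestroyed blocks toggling, but nothing in these graphs sets it or CurrentRot.
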(event `self.TriggerVolume.OnComponentBeginOverlap`
  (params (OtherActor :type "Actor Object Reference") (OtherComp :type "PrimitiveComponent Object Reference") (OtherBodyIndex :type Integer) (bFromSweep :type Boolean) (SweepResult :type "HitResult Structure (by ref)"))
  (`self.EnableInput` (`GameplayStatics.GetPlayerController` 0)))

(event `self.TriggerVolume.OnComponentEndOverlap`
  (params (OtherActor :type "Actor Object Reference") (OtherComp :type "PrimitiveComponent Object Reference") (OtherBodyIndex :type Integer))
  (`self.DisableInput` (`GameplayStatics.GetPlayerController` 0)))

(event `InputAction|ActionButton`
  (params (Key :type "Key Structure" :default "AnyKey"))
  (:`Pressed`
    (if (`self.IsDestroyed`)
      _
      (elif (`self.DoorPos`)
        (set `self.DoorPos` false)
        (bind (_direction _driver) (`Timeline|Timeline_0` :!label _label)
          (:`Update`
            (`self.K2_SetActorRelativeRotation` (`KismetMathLibrary.MakeRotator` 0.0 0.0 (+ _driver (`self.currentRot`))))))
        (else
          (set `self.DoorPos` true)
          (goto _label :!via `Reverse`))))))

(fn `UserConstructionScript`)